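; An actor component that tracks an actor's current and maximum health and a descriptive health status.
; Heal and TakeDamage add to or subtract from CurrentHealth without clamping or refreshing the status.
; A separate CheckHealth function maps health thresholds to a status from full to dead, clamping overflow and underflow.
; The event graph is empty, so nothing in this asset calls CheckHealth.
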(event EventBeginPlay)

(event EventTick
  (params (DeltaSeconds :type Float%20%28single-precision%29)))

(fn CheckHealth
  ;[1 1 1] Health Full
  (if (>= (Variables|Default|GetCurrentHealth) (Variables|Default|GetMaxHealth))
    (Variables|Default|SetHealthStatus "Health Full")
    ;;[1 1 1] Health Overflow Safety
    (Variables|Default|SetCurrentHealth (Variables|Default|GetMaxHealth))
    (else
      ;[0.9352 1 0.35] 100% > Health >= 75%
      (if (>= (Variables|Default|GetCurrentHealth) (* (Variables|Default|GetMaxHealth) 0.75))
        (Variables|Default|SetHealthStatus "Slight Damage")
        (else
          ;[1 0.7416 0.4547] 75% > Health > 50%
          (if (>= (Variables|Default|GetCurrentHealth) (* (Variables|Default|GetMaxHealth) 0.5))
            (Variables|Default|SetHealthStatus "Moderate Damage")
            (else
              ;[1 0.4557 0.3899] 50% > Health > 0
              (if (and (< (Variables|Default|GetCurrentHealth) (* (Variables|Default|GetMaxHealth) 0.5)) (> (Variables|Default|GetCurrentHealth) 0.0))
                (Variables|Default|SetHealthStatus "Severe Damage")
                (else
                  ;[1 0.2025 0.1766] Health <= 0
                  (if (<= (Variables|Default|GetCurrentHealth) 0.0)
                    (Variables|Default|SetHealthStatus "Dead")
                    ;;[1 1 1] Health Underflow Safety
                    (Variables|Default|SetCurrentHealth 0.0)))))))))))

(fn Heal
  (params (HealAmount :type Float%20%28double-precision%29))
  (Variables|Default|SetCurrentHealth (+ HealAmount (Variables|Default|GetCurrentHealth))))

(fn TakeDamage
  (params (Damage_amount :type Float%20%28double-precision%29))
  (Variables|Default|SetCurrentHealth (- (Variables|Default|GetCurrentHealth) Damage_amount)))