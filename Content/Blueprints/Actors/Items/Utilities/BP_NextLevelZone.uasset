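; BP_NextLevelZone is a level exit that loads a named level when an explorer character enters it with enough keys.
; On overlap of its EndZone, it pushes the character's currency, keys and current health to the dungeon game instance before opening the level, otherwise printing a not-enough-keys message.
; The construction script calls a debug helper, marked for deletion before shipping, that keeps the zone visible in game.
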(event OnComponentBeginOverlap(EndZone)
  (params (OverlappedComponent :type Primitive%20Component%20Object%20Reference) (OtherActor :type Actor%20Object%20Reference) (OtherComp :type Primitive%20Component%20Object%20Reference) (OtherBodyIndex :type Integer) (bFromSweep :type Boolean) (SweepResult :type Hit%20Result%20Structure%20%28by%20ref%29))
  (bind _asbp_explorer_character (Utilities|Casting|CastToBP_ExplorerCharacter OtherActor))
  (if (>= (Variables|/Game/Blueprints/Actors/Characters/Players/BP_ExplorerCharacter.BP_ExplorerCharacter_C|GetKeys _asbp_explorer_character) (Variables|Default|GetKeysRequirement))
    (Default|PushVariables (Variables|Default|GetGIRef) (Variables|/Game/Blueprints/Actors/Characters/Players/BP_ExplorerCharacter.BP_ExplorerCharacter_C|GetCurrency _asbp_explorer_character) (Variables|/Game/Blueprints/Actors/Characters/Players/BP_ExplorerCharacter.BP_ExplorerCharacter_C|GetKeys _asbp_explorer_character) (Variables|/Game/Blueprints/Components/ActorComponents/AC_HealthComponent.AC_HealthComponent_C|GetCurrentHealth (Variables|/Game/Blueprints/Actors/Characters/Players/BP_ExplorerCharacter.BP_ExplorerCharacter_C|GetAC_HealthComponent _asbp_explorer_character)))
    (Game|OpenLevel(byName) (Variables|Default|GetLevelName))
    (else
      (Development|PrintString "Not Enough Keys" true true "(R=1.000000,G=0.011438,B=0.055220,A=1.000000)" 5.0))))

(event EventBeginPlay
  (bind _asbp_mystery_dungeon_gi (Utilities|Casting|CastToBP_MysteryDungeon_GI (Game|GetGameInstance)))
  (Variables|Default|SetGIRef _asbp_mystery_dungeon_gi))

(fn ConstructionScript
  (CallFunction|DELETEBEFORESHIPPING (Variables|Default|GetEndZone)))

(fn DELETEBEFORESHIPPING
  (params (self2 :type Scene%20Component%20Object%20Reference))
  (Development|SetHiddeninGame self2 false false))