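; BP_Dmg_Over_Time is a damage zone actor that steadily hurts the explorer character while it stands inside.
; Entering Health_Zone stores the BP_ExplorerCharacter and starts damage through its ACHealthComponent.
; The damage event re-arms a one-second timer on itself, so the first hit is immediate and repeats every second.
; Leaving the zone clears the player reference and invalidates the timer.
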(event OnComponentBeginOverlap(Health_Zone)
  (params (OverlappedComponent :type Primitive%20Component%20Object%20Reference) (OtherActor :type Actor%20Object%20Reference) (OtherComp :type Primitive%20Component%20Object%20Reference) (OtherBodyIndex :type Integer) (bFromSweep :type Boolean) (SweepResult :type Hit%20Result%20Structure%20%28by%20ref%29))
  (bind _asbp_explorer_character (Utilities|Casting|CastToBP_ExplorerCharacter OtherActor))
  (Variables|Default|SetPlayerRef _asbp_explorer_character)
  (CallFunction|StartDamage))

(event OnComponentEndOverlap(Health_Zone)
  (params (OverlappedComponent :type Primitive%20Component%20Object%20Reference) (OtherActor :type Actor%20Object%20Reference) (OtherComp :type Primitive%20Component%20Object%20Reference) (OtherBodyIndex :type Integer))
  (Utilities|Casting|CastToBP_ExplorerCharacter OtherActor)
  (Variables|Default|SetPlayerRef 0)
  (CallFunction|StopDamage))

(event Custom|Start_Damage
  (bind _returnvalue (Utilities|Time|SetTimerbyEvent (delegate Custom|Start_Damage) 1.0))
  (Default|TakeDamage (Variables|/Game/Blueprints/Actors/Characters/Players/BP_ExplorerCharacter.BP_ExplorerCharacter_C|GetAC_HealthComponent (Variables|Default|GetPlayerRef)) 2.0))

(event Custom|Stop_Damage
  (Utilities|Time|ClearandInvalidateTimerbyHandle (stale Custom|Start_Damage _returnvalue)))

(event EventBeginPlay)

(event Collision|EventActorBeginOverlap
  (params (OtherActor :type Actor%20Object%20Reference)))

(event EventTick
  (params (DeltaSeconds :type Float%20%28single-precision%29)))

(fn ConstructionScript)