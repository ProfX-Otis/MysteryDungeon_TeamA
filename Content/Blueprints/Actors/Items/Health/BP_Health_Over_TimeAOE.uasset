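; Area-of-effect health pickup actor that heals a BP_ExplorerCharacter over time while it stands inside the Health_Zone.
; Entering the zone stores the player and starts a healing event that heals a fixed amount through its ACHealthComponent and re-arms a one-second timer on itself.
; Leaving the zone clears the player reference and invalidates that timer to stop the healing.
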(event OnComponentBeginOverlap(Health_Zone)
  (params (OverlappedComponent :type Primitive%20Component%20Object%20Reference) (OtherActor :type Actor%20Object%20Reference) (OtherComp :type Primitive%20Component%20Object%20Reference) (OtherBodyIndex :type Integer) (bFromSweep :type Boolean) (SweepResult :type Hit%20Result%20Structure%20%28by%20ref%29))
  (bind _asbp_explorer_character (Utilities|Casting|CastToBP_ExplorerCharacter OtherActor))
  (Variables|Default|SetPlayerRef _asbp_explorer_character)
  (CallFunction|StartHealing))

(event OnComponentEndOverlap(Health_Zone)
  (params (OverlappedComponent :type Primitive%20Component%20Object%20Reference) (OtherActor :type Actor%20Object%20Reference) (OtherComp :type Primitive%20Component%20Object%20Reference) (OtherBodyIndex :type Integer))
  (Utilities|Casting|CastToBP_ExplorerCharacter OtherActor)
  (Variables|Default|SetPlayerRef 0)
  (CallFunction|StopHealing))

(event Custom|Start_Healing
  (bind _returnvalue (Utilities|Time|SetTimerbyEvent (delegate Custom|Start_Healing) 1.0))
  (Default|Heal (Variables|/Game/Blueprints/Actors/Characters/Players/BP_ExplorerCharacter.BP_ExplorerCharacter_C|GetAC_HealthComponent (Variables|Default|GetPlayerRef)) 4.0))

(event Custom|Stop_Healing
  (Utilities|Time|ClearandInvalidateTimerbyHandle (stale Custom|Start_Healing _returnvalue)))

(event EventBeginPlay)

(event Collision|EventActorBeginOverlap
  (params (OtherActor :type Actor%20Object%20Reference)))

(event EventTick
  (params (DeltaSeconds :type Float%20%28single-precision%29)))

(fn ConstructionScript)