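; Enemy character that patrols target actors, chases or searches for BP_ExplorerCharacter, and triggers the player's death sequence on overlapping EnemyCaptureZone.
; Non-aborted move completions advance the looping patrol after a pause.
; AI Perception updates on a non-hidden player start a running chase when sensed, or a move to the last stimulus location when lost, with DetectionLight color showing the state.
; The construction script unhides both capture zones as debug left to remove before shipping.
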(event OnTargetPerceptionUpdated(AIPerception)
  (params (Actor :type Actor%20Object%20Reference) (Stimulus :type AI%20Stimulus%20Structure))
  ;[0.9859 0.645 1] Perceive Player
  (bind _asbp_explorer_character (Utilities|Casting|CastToBP_ExplorerCharacter Actor))
  (if (not (Variables|/Game/Blueprints/Actors/Characters/Players/BP_ExplorerCharacter.BP_ExplorerCharacter_C|GetHidden _asbp_explorer_character))
    (if (.bsuccessfullysensed Stimulus)
      (CallFunction|ChasePlayer _asbp_explorer_character)
      (else
        (CallFunction|SearchforPlayer (.stimuluslocation Stimulus))))))

(event OnComponentBeginOverlap(EnemyCaptureZone)
  (params (OverlappedComponent :type Primitive%20Component%20Object%20Reference) (OtherActor :type Actor%20Object%20Reference) (OtherComp :type Primitive%20Component%20Object%20Reference) (OtherBodyIndex :type Integer) (bFromSweep :type Boolean) (SweepResult :type Hit%20Result%20Structure%20%28by%20ref%29))
  (bind _asbp_explorer_character (Utilities|Casting|CastToBP_ExplorerCharacter OtherActor))
  (Default|PlayerDeathSequence _asbp_explorer_character))

(event Custom|InitializePatrol
  ;[0.4999 1 0.5798] Init Patrol
  (EventDispatchers|BindEventtoReceiveMoveCompleted (AI|GetAIController self) (delegate Custom|MoveCompleted))
  (Utilities|MovetoNextTarget))

(event Custom|MoveCompleted
  (params (RequestID :type AI%20Request%20ID%20Structure) (Result :type EPathFollowingResult%20Enum :default "Success"))
  ;[0.4999 1 0.5798] Init Patrol
  (switch Utilities|FlowControl|Switch|SwitchonEPathFollowingResult Result
    (:Success
      _)
    (:Blocked
      _)
    (:OffPath
      _)
    (:Invalid
      _))
  (Utilities|MovetoNextTarget))

(event EventBeginPlay
  (CallFunction|InitializePatrol))

(fn ConstructionScript
  (CallFunction|DELETEBEFORESHIPPING))

(fn DELETEBEFORESHIPPING
  (Development|SetHiddeninGame (Variables|Default|GetPlayerCaptureZone) false false))

(fn InitializeDetection
  (Rendering|Components|Light|SetLightColor (Variables|Default|GetDetectionLight) (Variables|Default|GetPatrolColor) true)
  (Variables|/Script/Engine.CharacterMovementComponent|SetMaxWalkSpeed (Variables|Character|GetCharacterMovement) (Variables|Default|GetWalkSpeed)))

(fn LocateTargetMove
  (bind _self self)
  (bind _patroltargets (Variables|Default|GetPatrolTargets))
  (bind _returnvalue (AI|GetAIController _self))
  (bind _result (Math|Integer|IncrementInt (Variables|Default|GetPatrolTargetIndex))
    (:%20%20
      (Utilities|IsValid (Utilities|Array|Get(acopy) _patroltargets (Math|Integer|%(Integer) _result (Utilities|Array|Length _patroltargets)))
        (:Is%20Valid
          (Utilities|IsValid _returnvalue
            (:Is%20Valid
              (AI|Navigation|MovetoActor _returnvalue (Utilities|Array|Get(acopy) _patroltargets (Math|Integer|%(Integer) _result (Utilities|Array|Length _patroltargets))) -1.0 true true true 0))))))))

(fn ChasePlayer
  (params (Goal :type Actor%20Object%20Reference))
  (AI|Navigation|SimpleMovetoActor (AI|GetAIController self) Goal)
  (Variables|/Script/Engine.CharacterMovementComponent|SetMaxWalkSpeed (Variables|Character|GetCharacterMovement) (Variables|Default|GetRunSpeed))
  (Rendering|Components|Light|SetLightColor (Variables|Default|GetDetectionLight) (Variables|Default|GetChaseColor) true))

(fn SearchforPlayer
  (params (Destination :type Vector))
  (bind _returnvalue (AI|Navigation|MovetoLocation (AI|GetAIController self) Destination -1.0 true true false true 0))
  (switch Utilities|FlowControl|Switch|SwitchonEPathFollowingRequestResult _returnvalue
    (:RequestSuccessful
      (Rendering|Components|Light|SetLightColor (Variables|Default|GetDetectionLight) (Variables|Default|GetSearchColor) true))))